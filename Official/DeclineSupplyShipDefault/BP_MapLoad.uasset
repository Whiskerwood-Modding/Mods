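; Map-load mod actor that preselects "Refuse supplies" whenever a supply trade ship docks at the main dock, unless its mod option is Off.
; After loading, it binds to the FactionDock's ship-change event and creates an off-screen supply trader panel.
; A delayed check, retried briefly, finds the reject choice and sends chooseSupplyPackage through that panel, imitating a HUD action.
; A non-empty debug config file enables logging.
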(event `self.ReceiveBeginPlay`
  (add `ModAPI.onLoadingFinished` (`ModAPI.GetModAPI`) (delegate `OnLoaded`)))

(event `OnLoaded`
  (bind _returnvalue (`ModAPI.ReadModTextFile` (`ModAPI.GetModAPI`) "DeclineSupplyShipDefaultConfig" "debug"))
  (set `self.Debug` (not (`KismetStringLibrary.IsEmpty` _returnvalue)))
  (bind (_out_isvalid _returnvalue_2) (`ArcoSystems.GetArcoSys`))
  (set `self.Sys` _returnvalue_2)
  (bind _returnvalue_3 (`ArcoSystems.GetPrimaryDockActor` _returnvalue_2))
  (bind _returnvalue_4 (`self.GetComponentByClass` _returnvalue_3 "/Script/ProjectArco.FactionDock"))
  (if (`KismetSystemLibrary.IsValid` _returnvalue_4)
    (add `FactionDock.DockedShipChanged` _returnvalue_4 (delegate `OnShipChanged`))
    (if (`self.Debug`)
      (`ModAPI.LogMessage` (`ModAPI.GetModAPI`) "DeclineSupplyShipDefault 1.0 (v8): main dock found, waiting for ships" true))
    (elif (`self.Debug`)
      (`ModAPI.LogMessage` (`ModAPI.GetModAPI`) (`KismetStringLibrary.Concat_StrStr` (`KismetStringLibrary.Concat_StrStr` "DeclineSupplyShipDefault 1.0 (v8): NO FactionDock found, main dock actor = ") (`KismetSystemLibrary.GetDisplayName` _returnvalue_3)) true)))
  (bind _returnvalue_5 (`|CreateWidget` "/Script/ProjectArco.DockedBoatPanel_SupplyTrader" (`GameplayStatics.GetPlayerController` 0)))
  (set `self.Panel` _returnvalue_5))

(event `OnShipChanged`
  (params (shipTypeAtDock :type "EShipType Enum" :default "TAX_SHIP"))
  (bind _returnvalue (`KismetStringLibrary.Conv_ByteToString` shipTypeAtDock))
  (if (`self.Debug`)
    (`ModAPI.LogMessage` (`ModAPI.GetModAPI`) (`KismetStringLibrary.Concat_StrStr` (`KismetStringLibrary.Concat_StrStr` (`KismetStringLibrary.Concat_StrStr` "DeclineSupplyShipDefault: ship at main dock changed, type ") _returnvalue) " (2 supply embark, 3 supply trade, 6 none)") true))
  (set `self.ShipType` (`KismetMathLibrary.Conv_ByteToInt` shipTypeAtDock))
  (bind _returnvalue_2 (`ModAPI.ReadModOptionValue` (`ModAPI.GetModAPI`) "DeclineSupplyShipDefault_On" "On"))
  (if (and (not (== _returnvalue_2 "Off")) (`KismetStringLibrary.EqualEqual_StrStr` _returnvalue "3"))
    (set `self.Tries` 3)
    (set `self.RetryPending` true)
    (`KismetSystemLibrary.K2_SetTimer` self "OnCheck" 0.5)))

(event `OnCheck`
  (bind _curidx (`self.CurIdx`))
  (bind _panel (`self.Panel`))
  (bind _rejectidx (`self.RejectIdx`))
  (bind _sys (`self.Sys`))
  (bind ((`shipType` _shiptype) (`shipState` _shipstate) (`asSupplyShip` _assupplyship)) (break `DockableShipData` (`ArcoSystems.GetCurrentlyDockedShipInfo` _sys)))
  (bind ((`choices` _choices) (`choiceIdx` _choiceidx)) (break `SupplyShipState` _assupplyship))
  (set `self.RetryPending` false)
  (if (`KismetSystemLibrary.IsValid` _sys)
    (set `self.Choices` _choices)
    (set `self.CurIdx` _choiceidx)
    (set `self.RejectIdx` -1)
    (for (_array_element _array_index) (`self.Choices`)
      (if (`.isRejectChoice` (break `SupplyShipChoice` _array_element))
        (set `self.RejectIdx` _array_index)))
    (if (`self.Debug`)
      (`ModAPI.LogMessage` (`ModAPI.GetModAPI`) (`KismetStringLibrary.Concat_StrStr` (`KismetStringLibrary.Concat_StrStr` (`KismetStringLibrary.Concat_StrStr` (`KismetStringLibrary.Concat_StrStr` (`KismetStringLibrary.Concat_StrStr` (`KismetStringLibrary.Concat_StrStr` (`KismetStringLibrary.Concat_StrStr` (`KismetStringLibrary.Concat_StrStr` (`KismetStringLibrary.Concat_StrStr` (`KismetStringLibrary.Concat_StrStr` (`KismetStringLibrary.Concat_StrStr` (`KismetStringLibrary.Concat_StrStr` "DeclineSupplyShipDefault:   docked ship type ") (`KismetStringLibrary.Conv_ByteToString` _shiptype)) ", state ") (`KismetStringLibrary.Conv_ByteToString` _shipstate)) ", choices ") (`KismetStringLibrary.Conv_IntToString` (`KismetArrayLibrary.Array_Length` (`self.Choices`)))) ", selected ") (`KismetStringLibrary.Conv_IntToString` _curidx)) ", reject choice ") (`KismetStringLibrary.Conv_IntToString` _rejectidx)) ", tries left ") (`KismetStringLibrary.Conv_IntToString` (`self.Tries`))) true))
    (if (>= _rejectidx 0)
      (if (== _rejectidx _curidx)
        (if (`self.Debug`)
          (`ModAPI.LogMessage` (`ModAPI.GetModAPI`) "DeclineSupplyShipDefault:   Refuse supplies already selected" true))
        (elif (`KismetSystemLibrary.IsValid` _panel)
          (`ArcoWidgetBase.ReceiveHudAction` _panel (make `HudAction` :`action` "chooseSupplyPackage" :`paramInt` _rejectidx))
          (if (`self.Debug`)
            (`ModAPI.LogMessage` (`ModAPI.GetModAPI`) (`KismetStringLibrary.Concat_StrStr` (`KismetStringLibrary.Concat_StrStr` (`KismetStringLibrary.Concat_StrStr` (`KismetStringLibrary.Concat_StrStr` "DeclineSupplyShipDefault:   sent chooseSupplyPackage ") (`KismetStringLibrary.Conv_IntToString` _rejectidx)) ", selected now ") (`KismetStringLibrary.Conv_IntToString` (`.choiceIdx` (break `SupplyShipState` (`.asSupplyShip` (break `DockableShipData` (`ArcoSystems.GetCurrentlyDockedShipInfo` _sys))))))) true))
          (elif (`self.Debug`)
            (`ModAPI.LogMessage` (`ModAPI.GetModAPI`) "DeclineSupplyShipDefault:   invisible supply panel missing" true))))
      (else
        (set `self.Tries` (- (`self.Tries`) 1))
        (if (and (> (`self.Tries`) 0) (not (`self.RetryPending`)))
          (set `self.RetryPending` true)
          (`KismetSystemLibrary.K2_SetTimer` self "OnCheck" 1.0)
          (if (`self.Debug`)
            (`ModAPI.LogMessage` (`ModAPI.GetModAPI`) "DeclineSupplyShipDefault:   no Refuse supplies choice yet, checking again in 1.0 s" true))
          (elif (`self.Debug`)
            (`ModAPI.LogMessage` (`ModAPI.GetModAPI`) "DeclineSupplyShipDefault:   no Refuse supplies choice, giving up" true)))))
    (elif (`self.Debug`)
      (`ModAPI.LogMessage` (`ModAPI.GetModAPI`) "DeclineSupplyShipDefault:   ArcoSystems not valid" true))))

(fn `UserConstructionScript`)