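; Main-menu loader for the LongerDays mod that lets players set day and night lengths through mod options.
; On BeginPlay it adds English strings, registers both options with localized text, then applies saved values; option changes reapply them.
; SetNewDayLengths overwrites SystemTunes rows for phase, day, year and dependent timers via the mod API.
; It also rescales non-zero minimum maintenance intervals in GridActors to the day length.
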(event `self.ReceiveBeginPlay`
  (add `ModAPI.onOptionChanged` (`ModAPI.GetModAPI`) (`|CreateDelegate` :!event `OnOptionChanged`))
  (`self.Add New Strings`)
  (`KismetSystemLibrary.Delay` 0.5)
  (`self.Register Day Options`)
  (`self.Register Night Options`)
  (bind _returnvalue (`ModAPI.ReadModOptionValue` (`ModAPI.GetModAPI`) (`self.DayLenOptionId`) (`self.DayDefault`)))
  (bind _returnvalue_2 (`ModAPI.ReadModOptionValue` (`ModAPI.GetModAPI`) (`self.NightLenOptionId`) (`self.NightDefault`)))
  (`self.Set New Day Lengths` _returnvalue _returnvalue_2))

(event `OnOptionChanged`
  (params (optionId :type String) (Value :type String))
  (if (`KismetStringLibrary.EqualEqual_StrStr` optionId "settings.language")
    (`self.Register Day Options`)
    (elif (`KismetStringLibrary.EqualEqual_StrStr` optionId (`self.DayLenOptionId`))
      (bind _output_get (set `self.DayLen` Value))
      (`self.Set New Day Lengths` _output_get (stale _output_get_2) :!label _label)
      (elif (`KismetStringLibrary.EqualEqual_StrStr` optionId (`self.NightLenOptionId`))
        (bind _output_get_2 (set `self.NightLen` Value))
        (goto _label)))))

(fn `Add New Strings`
  (bind _returnvalue (`ModAPI.GetModAPI`))
  (bind _nightlenoptionid (`self.NightLenOptionId`))
  (bind _daylenoptionid (`self.DayLenOptionId`))
  (`ModAPI.AddNewStrings` _returnvalue "en" (`|MakeMap` (`KismetStringLibrary.Conv_StringToName` (`KismetStringLibrary.Concat_StrStr` "setting." _daylenoptionid ".name")) (`self.DayLenName`) (`KismetStringLibrary.Conv_StringToName` (`KismetStringLibrary.Concat_StrStr` "setting." _daylenoptionid ".description")) (`self.DayLenDesc`)))
  (`ModAPI.AddNewStrings` _returnvalue "en" (`|MakeMap` (`KismetStringLibrary.Conv_StringToName` (`KismetStringLibrary.Concat_StrStr` "setting." _nightlenoptionid ".name")) (`self.NightLenName`) (`KismetStringLibrary.Conv_StringToName` (`KismetStringLibrary.Concat_StrStr` "setting." _nightlenoptionid ".description")) (`self.NightLenDesc`))))

(fn `Get Localized Option`
  (params (OptionId :type String) (DefaultName :type String) (DefaultDesc :type String))
  (returns (Name :type String) (Description :type String))
  (bind _returnvalue (`Backbone.GetLocManager`))
  (bind _returnvalue_2 (`LocManager.GetWordFromKey` _returnvalue (`KismetStringLibrary.Conv_StringToName` (`KismetStringLibrary.Concat_StrStr` "setting." OptionId ".description"))))
  (bind _returnvalue_3 (`LocManager.GetWordFromKey` _returnvalue (`KismetStringLibrary.Conv_StringToName` (`KismetStringLibrary.Concat_StrStr` "setting." OptionId ".name"))))
  (bind _returnvalue_4 (`KismetStringLibrary.IsEmpty` _returnvalue_2))
  (if (`KismetStringLibrary.IsEmpty` _returnvalue_3)
    (if _returnvalue_4
      (return DefaultName DefaultDesc)
      (else
        (return DefaultName _returnvalue_2)))
    (elif _returnvalue_4
      (return _returnvalue_3 DefaultDesc)
      (else
        (return _returnvalue_3 _returnvalue_2)))))

(fn `Log`
  (params (Message :type String))
  (if (`self.Log Messages?`)
    (`ModAPI.LogMessage` (`ModAPI.GetModAPI`) (`KismetStringLibrary.Concat_StrStr` "[" (`self.Mod Name`) "] " Message) true)))

(fn `Register Day Options`
  (bind _daylenoptionid (`self.DayLenOptionId`))
  (bind (_name _description) (`self.Get Localized Option` _daylenoptionid (`self.DayLenName`) (`self.DayLenDesc`)))
  (bind _returnvalue (`ModAPI.RegisterModOptions` (`ModAPI.GetModAPI`) _daylenoptionid _name (`self.DayOptionsValues`) (`self.DayDefault`) _description))
  (`self.Log` (`KismetStringLibrary.Conv_BoolToString` _returnvalue)))

(fn `Register Night Options`
  (bind _nightlenoptionid (`self.NightLenOptionId`))
  (bind (_name _description) (`self.Get Localized Option` _nightlenoptionid (`self.NightLenName`) (`self.NightLenDesc`)))
  (bind _returnvalue (`ModAPI.RegisterModOptions` (`ModAPI.GetModAPI`) _nightlenoptionid _name (`self.NightOptionsValues`) (`self.NightDefault`) _description))
  (`self.Log` (`KismetStringLibrary.Conv_BoolToString` _returnvalue)))

(fn `Set New Day Lengths`
  (params (`Day Minutes` :type String) (`Night Minutes` :type String))
  (locals (DaySecondsFloat :type "Float (double-precision)") (NightSecondsFloat :type "Float (double-precision)") (MaintLimitMult :type "Float (double-precision)" :default 2.4) (HardLaborInterval :type "Float (double-precision)" :default 10.5) (BeautyInterval :type "Float (double-precision)" :default 7.0) (MinMaintIntervalMult :type "Float (double-precision)" :default 17.1))
  (bind _returnvalue (`ModAPI.GetModAPI`))
  (bind _daysecondsfloat (`local.DaySecondsFloat`))
  (bind _returnvalue_2 (+ (`local.NightSecondsFloat`) _daysecondsfloat))
  (bind _returnvalue_3 (`KismetStringLibrary.Conv_DoubleToString` _returnvalue_2))
  (bind _returnvalue_4 (`KismetStringLibrary.Conv_DoubleToString` _returnvalue_2))
  (bind _output_get (set `self.DayLen` `Day Minutes`))
  (bind _output_get_2 (set `self.NightLen` `Night Minutes`))
  (bind _output_get_3 (set `local.DaySecondsFloat` (* (`KismetStringLibrary.Conv_StringToDouble` _output_get) 60.0)))
  (bind _returnvalue_5 (`KismetStringLibrary.Conv_DoubleToString` _output_get_3))
  (`self.Log` _returnvalue_5)
  (bind _returnvalue_6 (`ModAPI.WriteDataTableValue` _returnvalue "SystemTunes" "basePhaseLen_Day" "floatValue" _returnvalue_5))
  (`self.Log` (`KismetStringLibrary.Conv_BoolToString` _returnvalue_6))
  (bind _output_get_4 (set `local.NightSecondsFloat` (* (`KismetStringLibrary.Conv_StringToDouble` _output_get_2) 60.0)))
  (bind _returnvalue_7 (`KismetStringLibrary.Conv_DoubleToString` _output_get_4))
  (`self.Log` _returnvalue_7)
  (bind _returnvalue_8 (`ModAPI.WriteDataTableValue` _returnvalue "SystemTunes" "basePhaseLen_Night" "floatValue" _returnvalue_7))
  (`self.Log` (`KismetStringLibrary.Conv_BoolToString` _returnvalue_8))
  (`self.Log` _returnvalue_4)
  (bind _returnvalue_9 (`ModAPI.WriteDataTableValue` _returnvalue "SystemTunes" "totalDayLen_Derived" "floatValue" _returnvalue_4))
  (`self.Log` (`KismetStringLibrary.Conv_BoolToString` _returnvalue_9))
  (bind _returnvalue_10 (`ModAPI.WriteDataTableValue` _returnvalue "SystemTunes" "maintenanceTimeLimit" "floatValue" (`KismetStringLibrary.Conv_DoubleToString` (* (`local.MaintLimitMult`) _daysecondsfloat))))
  (`self.Log` (`KismetStringLibrary.Conv_BoolToString` _returnvalue_10))
  (bind _returnvalue_11 (`ModAPI.ReadDataTableValue` _returnvalue "SystemTunes" "baseDaysYear" "floatValue"))
  (`self.Log` _returnvalue_11)
  (bind _returnvalue_12 (`KismetStringLibrary.Conv_DoubleToString` (* (`KismetStringLibrary.Conv_StringToDouble` _returnvalue_11) _returnvalue_2)))
  (`self.Log` _returnvalue_12)
  (bind _returnvalue_13 (`ModAPI.WriteDataTableValue` _returnvalue "SystemTunes" "SecondsPerYear" "floatValue" _returnvalue_12))
  (`self.Log` (`KismetStringLibrary.Conv_BoolToString` _returnvalue_13))
  (`self.Log` _returnvalue_3)
  (bind _returnvalue_14 (`ModAPI.WriteDataTableValue` _returnvalue "SystemTunes" "TemperatureChangePeriod" "floatValue" _returnvalue_3))
  (`self.Log` (`KismetStringLibrary.Conv_BoolToString` _returnvalue_14))
  (bind _returnvalue_15 (`ModAPI.WriteDataTableValue` _returnvalue "SystemTunes" "hardlabor_triggerInterval" "floatValue" (`KismetStringLibrary.Conv_DoubleToString` (/ (`local.DaySecondsFloat`) (`local.HardLaborInterval`)))))
  (`self.Log` (`KismetStringLibrary.Conv_BoolToString` _returnvalue_15))
  (bind _returnvalue_16 (`ModAPI.WriteDataTableValue` _returnvalue "SystemTunes" "BeautyCooldown" "floatValue" (`KismetStringLibrary.Conv_DoubleToString` (/ (`local.DaySecondsFloat`) (`local.BeautyInterval`)))))
  (`self.Log` (`KismetStringLibrary.Conv_BoolToString` _returnvalue_16))
  (bind _outrownames (`DataTableFunctionLibrary.GetDataTableRowNames` "/Game/Data/GridactorDefs_Sync.GridactorDefs_Sync"))
  (for _array_element _outrownames
    (bind _returnvalue_17 (`ModAPI.ReadDataTableValue` _returnvalue "GridActors" _array_element "minMaintenanceInterval"))
    (if (!= (`KismetStringLibrary.Conv_StringToInt` _returnvalue_17) 0)
      (`ModAPI.WriteDataTableValue` _returnvalue "GridActors" _array_element "minMaintenanceInterval" (`KismetStringLibrary.Conv_DoubleToString` (* (`local.DaySecondsFloat`) (`local.MinMaintIntervalMult`)))))))

(fn `UserConstructionScript`)