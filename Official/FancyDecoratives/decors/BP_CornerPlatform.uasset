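; BP_CornerPlatform is a decorative corner platform actor built entirely in its construction script, with no active event logic.
; It clears and refills two instanced mesh components, SupportRope and SupportNoRope, from separate transform arrays for supports with and without rope.
; It also adds a box component at each transform in CollisionBoxArr, so collision layout is data-driven alongside the instanced visuals.
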(fn `UserConstructionScript`
  (`InstancedStaticMeshComponent.ClearInstances` (`self.SupportRope`))
  (`InstancedStaticMeshComponent.ClearInstances` (`self.SupportNoRope`))
  (`InstancedStaticMeshComponent.AddInstances` (`self.SupportRope`) (`self.TransformArr`) false false true)
  (`InstancedStaticMeshComponent.AddInstances` (`self.SupportNoRope`) (`self.TransformArrNoRope`) false false true)
  (for _array_element (`self.CollisionBoxArr`)
    (`AddComponent|NODE_AddBoxComponent-1` :`RelativeTransform` _array_element)))