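; BP_Light is a decorative light from FancyDecoratives that lights up and spins while its Industry source is running.
; The Industry RunningChangedEvent stores the running state and switches two point lights and a spot light between full intensity and off.
; Tick yaws the Light component at a constant, frame-rate-independent speed while running and applies a zero rotation otherwise.
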(event `self.ReceiveBeginPlay`)

(event `self.ReceiveTick`
  (params (DeltaSeconds :type "Float (single-precision)"))
  (bind _light (`self.light`))
  (if (`self.running`)
    (`SceneComponent.K2_AddLocalRotation` _light (`KismetMathLibrary.MakeRotator` 0.0 0.0 (* DeltaSeconds 50.0)) false false)
    (else
      (`SceneComponent.K2_AddLocalRotation` _light (`KismetMathLibrary.MakeRotator` 0.0) false false))))

(event `self.Industry.runningChangedEvent`
  (params (IsRunning :type Boolean))
  (bind _output_get (set `self.running` IsRunning))
  (if _output_get
    (`LightComponent.SetIntensity` (`self.PointLight1`) 5000.0)
    (`LightComponent.SetIntensity` (`self.SpotLight`) 5000.0)
    (`LightComponent.SetIntensity` (`self.PointLight`) 5000.0)
    (else
      (`LightComponent.SetIntensity` (`self.PointLight1`) 0.0)
      (`LightComponent.SetIntensity` (`self.SpotLight`) 0.0)
      (`LightComponent.SetIntensity` (`self.PointLight`) 0.0))))

(fn `UserConstructionScript`)