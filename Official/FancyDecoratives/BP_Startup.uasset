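; Startup Blueprint for the Fancy Decoratives mod that registers its decorations and paths with the game on BeginPlay.
; It adds toolbar folders, then copies slot decorative and grid actor rows from mod tables into game tables, with icons.
; Writes go through the ModAPI as stringified values, and toolbar lists are extended by string splicing.
; Collected English names are added last; table dumps run after each grid actor.
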(event `self.ReceiveBeginPlay`
  (bind _fancygridactorstable (`self.FancyGridActorsTable`))
  (bind _fancyslotdecorativestable (`self.FancySlotDecorativesTable`))
  (`|ExecutionSequence`
    (:`then_0`
      (`self.AddModToolbar` "toolbar_fancydecor" "Fancy Decorations" "fancy_decoratives" "toolbar_decor" "/Game/Mods/FancyDecoratives/Icons/fancy_decors-100.fancy_decors-100")
      (`self.AddGroupToToolbar` "toolbar_fancydecor" "fancy_decor")
      (`self.AddModToolbar` "toolbar_fancypaths" "Fancy Paths" "fancy_paths" "toolbar_navigation" "/Game/Mods/FancyDecoratives/Icons/fancy_paths-100.fancy_paths-100")
      (`self.AddGroupToToolbar` "toolbar_fancypaths" "fancy_path"))
    (:`then_1`
      (bind _outrownames (`DataTableFunctionLibrary.GetDataTableRowNames` _fancyslotdecorativestable))
      (for _array_element _outrownames
        (bind _returnvalue (`|GetDataTableRow` _fancyslotdecorativestable _array_element)
          (:`then`
            (bind (_name _lockey _decorativeactor _desiredsubslot _pathingeffect _icon _enlocname) (break `/Game/Mods/FancyDecoratives/Data/S_FancySlotDecoratives` _returnvalue))
            (`self.Create New Slot Decorative` _name (make `SlotDecorative` _lockey _decorativeactor _desiredsubslot _pathingeffect) _icon _enlocname)))))
    (:`then_2`
      (bind _outrownames_2 (`DataTableFunctionLibrary.GetDataTableRowNames` _fancygridactorstable))
      (for _array_element_2 _outrownames_2
        (bind _returnvalue_2 (`|GetDataTableRow` _fancygridactorstable _array_element_2)
          (:`then`
            (bind (_name_2 _enlocname_2 _gridactor _stringkey _description _cost1 _ct1 _cost2 _ct2 _cost3 _ct3 _cost4 _ct4 _unlockprerequisite _toolbargroup _toolbargroupsort _usecustomicon _icon_2 _detailcue _supportedimprovements _structuretype _maxagents_contextual _ashousetier _asindustrydef _supportedindustryrecipes _minmaintenanceinterval _workercolor _limitone _custombuildcue _requiresconstruction _decortype _guildspecialty _hardlabor _industriallabor _tooltiptags _constructiontime _catalyst _norefund _randomlyrotate _refundrule _quality _variants _maxhealth _isdraggablewall) (break `/Game/Mods/FancyDecoratives/Data/S_FancyGridActors` _returnvalue_2))
            (`self.Create New Grid Actor` _name_2 (make `GridActorDefinition_MasterSyncFormat` _gridactor _stringkey _description _cost1 _ct1 _cost2 _ct2 _cost3 _ct3 _cost4 _ct4 _unlockprerequisite _toolbargroup _toolbargroupsort _usecustomicon _icon_2 _detailcue _supportedimprovements _structuretype _maxagents_contextual _ashousetier _asindustrydef _supportedindustryrecipes _maxhealth _minmaintenanceinterval _workercolor _limitone _custombuildcue _requiresconstruction _decortype _guildspecialty _hardlabor _industriallabor _tooltiptags _constructiontime _catalyst _norefund _randomlyrotate _refundrule _quality _variants _isdraggablewall) _icon_2 _enlocname_2)
            (`ModAPI.DumpAllDataTablesToLogFolder` (`ModAPI.GetModAPI`))))))
    (:`then_3`
      (bind _returnvalue_3 (`ModAPI.AddNewStrings` (`ModAPI.GetModAPI`) "en" (`self.Loc Strings`)))
      (if (not _returnvalue_3)
        (`self.Log Message` "failed to add to en table")))))

(fn `AddDividerToToolbar`
  (params (ToolbarRowName :type Name))
  (bind _returnvalue (`ModAPI.GetModAPI`))
  (`ModAPI.AddDataTable` _returnvalue "ToolbarDefinitions" "/Game/Data/ToolbarDefinitions.ToolbarDefinitions")
  (bind _returnvalue_2 (`ModAPI.ReadDataTableValue` _returnvalue "ToolbarDefinitions" ToolbarRowName "toolbarItems"))
  (`ModAPI.WriteDataTableValue` _returnvalue "ToolbarDefinitions" ToolbarRowName "toolbarItems" (`KismetStringLibrary.Concat_StrStr` (`KismetStringLibrary.LeftChop` _returnvalue_2 1) ",(ItemType=DIVIDER,itemKey=\"\",LocKey=\"\",Icon=None,HudAction=(action=\"\",paramString=\"\",paramName=\"\",paramInt=0,paramFloat=0.000000,paramGrid=(X=0,Y=0,Z=0),paramBool=False,paramVector=(X=0.000000,Y=0.000000,Z=0.000000)),categoryToOpen=\"\",gridActorGroup=\"\",gridActorName=\"\",RequiredUnlock=\"\",hideIfLocked=False,shouldTintIcon=True,hotkeyStr=\"\",showInWheel=False,customTooltip=\"\",associatedShortcutVerb=INVALID))")))

(fn `AddGroupToToolbar`
  (params (ToolbarRowName :type Name) (GroupName :type Name))
  (bind _returnvalue (`ModAPI.GetModAPI`))
  (`ModAPI.AddDataTable` _returnvalue "ToolbarDefinitions" "/Game/Data/ToolbarDefinitions.ToolbarDefinitions")
  (bind _returnvalue_2 (`ModAPI.ReadDataTableValue` _returnvalue "ToolbarDefinitions" ToolbarRowName "toolbarItems"))
  (`ModAPI.WriteDataTableValue` _returnvalue "ToolbarDefinitions" ToolbarRowName "toolbarItems" (`KismetStringLibrary.Concat_StrStr` (`KismetStringLibrary.LeftChop` _returnvalue_2 1) ",(ItemType=GRIDACTOR_GROUP,itemKey=\"\",LocKey=\"\",Icon=None,HudAction=(action=\"\",paramString=\"\",paramName=\"\",paramInt=0,paramFloat=0.000000,paramGrid=(X=0,Y=0,Z=0),paramBool=False,paramVector=(X=0.000000,Y=0.000000,Z=0.000000)),categoryToOpen=\"\",gridActorGroup=\"" (`KismetStringLibrary.Conv_NameToString` GroupName) "\",gridActorName=\"\",RequiredUnlock=\"\",hideIfLocked=False,shouldTintIcon=True,hotkeyStr=\"\",showInWheel=True,customTooltip=\"\",associatedShortcutVerb=INVALID))")))

(fn `AddModToolbar`
  (params (ToolbarRowName :type Name) (DisplayName :type String) (GroupName :type Name) (ToolbarTarget :type String) (icon :type "Texture2D Object Reference"))
  (locals (tempArray :type String) (ToolbarDefinitions :type "DataTable Object Reference"))
  (bind _returnvalue (`ModAPI.GetModAPI`))
  (`ModAPI.AddDataTable` _returnvalue "ToolbarDefinitions" "/Game/Data/ToolbarDefinitions.ToolbarDefinitions")
  (`ModAPI.AddDataTableRow` _returnvalue "ToolbarDefinitions" ToolbarRowName)
  (`ModAPI.WriteDataTableValue` _returnvalue "ToolbarDefinitions" ToolbarRowName "toolbarItems" (`KismetStringLibrary.Concat_StrStr` "((ItemType=GRIDACTOR_GROUP,itemKey=\"\",LocKey=\"" DisplayName "\",Icon=\"" (`KismetSystemLibrary.GetDisplayName` icon) "\",HudAction=(action=\"\",paramString=\"\",paramName=\"\",paramInt=0,paramFloat=0.000000,paramGrid=(X=0,Y=0,Z=0),paramBool=False,paramVector=(X=0.000000,Y=0.000000,Z=0.000000)),categoryToOpen=\"\",gridActorGroup=\"" (`KismetStringLibrary.Conv_NameToString` GroupName) "\",gridActorName=\"\",RequiredUnlock=\"\",hideIfLocked=False,shouldTintIcon=True,hotkeyStr=\"\",showInWheel=True,customTooltip=\"\",associatedShortcutVerb=INVALID))"))
  (bind _returnvalue_2 (`ModAPI.ReadDataTableValue` _returnvalue "ToolbarDefinitions" (`KismetStringLibrary.Conv_StringToName` ToolbarTarget) "toolbarItems"))
  (`ModAPI.WriteDataTableValue` _returnvalue "ToolbarDefinitions" (`KismetStringLibrary.Conv_StringToName` ToolbarTarget) "toolbarItems" (`KismetStringLibrary.Concat_StrStr` (`KismetStringLibrary.LeftChop` _returnvalue_2 1) ",(ItemType=FOLDER,itemKey=\"\",LocKey=\"" DisplayName "\",Icon=\"" (`KismetSystemLibrary.GetDisplayName` icon) "\",HudAction=(action=\"\",paramString=\"\",paramName=\"\",paramInt=0,paramFloat=0.000000,paramGrid=(X=0,Y=0,Z=0),paramBool=False,paramVector=(X=0.000000,Y=0.000000,Z=0.000000)),categoryToOpen=\"" (`KismetStringLibrary.Conv_NameToString` ToolbarRowName) "\",gridActorGroup=\"\",gridActorName=\"\",RequiredUnlock=\"\",hideIfLocked=False,shouldTintIcon=True,hotkeyStr=\"\",showInWheel=True,customTooltip=\"\",associatedShortcutVerb=INVALID))")))

(fn `Construct BP Ref`
  (params (ClassRef :type "Actor Class Reference"))
  (returns (OutName :type String))
  (bind _returnvalue_pathstring (`KismetSystemLibrary.BreakSoftClassPath` (`KismetSystemLibrary.GetSoftClassPath` ClassRef)))
  (return (`KismetStringLibrary.Concat_StrStr` "/Script/Engine.BlueprintGeneratedClass'" _returnvalue_pathstring "'")))

(fn `Construct Icon Ref`
  (params (Icon :type "Texture2D Object Reference"))
  (returns (Out :type String))
  (bind _returnvalue_pathstring (`KismetSystemLibrary.BreakSoftObjectPath` (`KismetSystemLibrary.GetSoftObjectPath` Icon)))
  (return (`KismetStringLibrary.Concat_StrStr` "/Script/Engine.Texture2D'" _returnvalue_pathstring "'")))

(fn `Convert AName to Stringified Value`
  (params (tooltipTags :type "Array of Name"))
  (returns (Out :type String))
  (locals (temparray :type String))
  (for _array_element tooltipTags
    (set `local.temparray` (`KismetStringLibrary.BuildString_Name` (`local.temparray`) "\"" _array_element "\",")))
  (return (`KismetStringLibrary.Concat_StrStr` "(" (`KismetStringLibrary.LeftChop` (`local.temparray`) 1) ")")))

(fn `Create New Grid Actor`
  (params (RowId :type Name) (Details :type "GridActorDefinition_MasterSyncFormat Structure") (Icon :type "Texture2D Object Reference") (name :type String))
  (`self.Write GridActors Row` RowId (make `GridActorDefinition_MasterSyncFormat` Details_GridActor Details_stringKey Details_Description Details_cost1 Details_ct1 Details_cost2 Details_ct2 Details_cost3 Details_ct3 Details_cost4 Details_ct4 Details_unlockPrerequisite Details_toolbarGroup Details_toolbarGroupSort Details_useCustomIcon Details_Icon Details_detailCue Details_SupportedImprovements Details_structureType Details_maxAgents_contextual Details_asHouseTier Details_asIndustryDef Details_supportedIndustryRecipes 0 Details_minMaintenanceInterval Details_workerColor Details_limitOne Details_customBuildCue Details_requiresConstruction Details_decorType Details_guildSpecialty Details_hardLabor Details_industrialLabor Details_TooltipTags Details_constructionTime Details_catalyst Details_norefund Details_randomlyRotate Details_refundRule Details_Quality Details_Variants))
  (`self.Write Icons Row` (make `IconDataRowBase` Icon) RowId)
  (`BlueprintMapLibrary.Map_Add` (`self.Loc Strings`) (`KismetStringLibrary.Conv_StringToName` Details_stringKey) name))

(fn `Create New Slot Decorative`
  (params (RowId :type Name) (Details :type "SlotDecorative Structure") (Icon :type "Texture2D Object Reference") (Name :type String))
  (`self.Write SlotDecoratives Row` RowId (make `SlotDecorative` Details_LocKey Details_decorativeActor Details_desiredSubSlot Details_pathingEffect))
  (`self.Write Icons Row` (make `IconDataRowBase` Icon) RowId)
  (`BlueprintMapLibrary.Map_Add` (`self.Loc Strings`) (`KismetStringLibrary.Conv_StringToName` Details_LocKey) Name))

(fn `Log Message`
  (params (Message :type String))
  (bind (_year _month _day _hour _minute _second _millisecond) (`KismetMathLibrary.BreakDateTime` (`KismetMathLibrary.Now`)))
  (if (`self.Enable Logging?`)
    (`ModAPI.LogMessage` (`ModAPI.GetModAPI`) (`KismetStringLibrary.Concat_StrStr` "[" (`KismetStringLibrary.Conv_IntToString` _year) "-" (`KismetStringLibrary.Conv_IntToString` _month) "-" (`KismetStringLibrary.Conv_IntToString` _day) " " (`KismetStringLibrary.Conv_IntToString` _hour) ":" (`KismetStringLibrary.Conv_IntToString` _minute) ":" (`KismetStringLibrary.Conv_IntToString` _second) "." (`KismetStringLibrary.Conv_IntToString` _millisecond) "] [" (`self.Mod Name`) "] " Message) false)))

(fn `UserConstructionScript`)

(fn `Write GridActors Row`
  (params (RowId :type Name) (GridActor :type "GridActorDefinition_MasterSyncFormat Structure"))
  (locals (GridActors :type Name :default "GridActors") (tooltipTags :type "Array of String") (actorMap :type "Map of Name to String"))
  (bind _returnvalue (`ModAPI.GetModAPI`))
  (bind _gridactors (`local.GridActors`))
  (bind _returnvalue_2 (`ModAPI.AddDataTableRow` _returnvalue _gridactors RowId))
  (if _returnvalue_2
    (bind _returnvalue_3 (`ModAPI.WriteDataTableValue` _returnvalue _gridactors RowId "gridActor" (`self.Construct BP Ref` GridActor_GridActor)))
    (if _returnvalue_3
      (bind _returnvalue_4 (`ModAPI.WriteDataTableValue` _returnvalue _gridactors RowId "stringKey" GridActor_stringKey))
      (if _returnvalue_4
        (bind _returnvalue_5 (`ModAPI.WriteDataTableValue` _returnvalue _gridactors RowId "Description" GridActor_Description))
        (if _returnvalue_5
          (bind _returnvalue_6 (`ModAPI.WriteDataTableValue` _returnvalue _gridactors RowId "cost1" (`KismetStringLibrary.Conv_NameToString` GridActor_cost1)))
          (if _returnvalue_6
            (bind _returnvalue_7 (`ModAPI.WriteDataTableValue` _returnvalue _gridactors RowId "ct1" (`KismetStringLibrary.Conv_IntToString` GridActor_ct1)))
            (if _returnvalue_7
              (bind _returnvalue_8 (`ModAPI.WriteDataTableValue` _returnvalue _gridactors RowId "cost2" (`KismetStringLibrary.Conv_NameToString` GridActor_cost2)))
              (if _returnvalue_8
                (bind _returnvalue_9 (`ModAPI.WriteDataTableValue` _returnvalue _gridactors RowId "ct2" (`KismetStringLibrary.Conv_IntToString` GridActor_ct2)))
                (if _returnvalue_9
                  (bind _returnvalue_10 (`ModAPI.WriteDataTableValue` _returnvalue _gridactors RowId "Variants" (`self.Convert AName to Stringified Value` GridActor_Variants)))
                  (if _returnvalue_10
                    (bind _returnvalue_11 (`ModAPI.WriteDataTableValue` _returnvalue _gridactors RowId "asIndustryDef" (`KismetStringLibrary.Conv_NameToString` GridActor_asIndustryDef)))
                    (if _returnvalue_11
                      (bind _returnvalue_12 (`ModAPI.WriteDataTableValue` _returnvalue _gridactors RowId "supportedIndustryRecipes" (`self.Convert AName to Stringified Value` GridActor_supportedIndustryRecipes)))
                      (if _returnvalue_12
                        (bind _returnvalue_13 (`ModAPI.WriteDataTableValue` _returnvalue _gridactors RowId "minMaintenanceInterval" (`KismetStringLibrary.Conv_IntToString` GridActor_minMaintenanceInterval)))
                        (if _returnvalue_13
                          (bind _returnvalue_14 (`ModAPI.WriteDataTableValue` _returnvalue _gridactors RowId "limitOne" (`KismetStringLibrary.Conv_BoolToString` GridActor_limitOne)))
                          (if _returnvalue_14
                            (bind _returnvalue_15 (`ModAPI.WriteDataTableValue` _returnvalue _gridactors RowId "customBuildCue" ""))
                            (if _returnvalue_15
                              (bind _returnvalue_16 (`ModAPI.WriteDataTableValue` _returnvalue _gridactors RowId "requiresConstruction" (`KismetStringLibrary.Conv_BoolToString` GridActor_requiresConstruction)))
                              (if _returnvalue_16
                                (bind _returnvalue_17 (`ModAPI.WriteDataTableValue` _returnvalue _gridactors RowId "guildSpecialty" (`KismetStringLibrary.Conv_NameToString` GridActor_guildSpecialty)))
                                (if _returnvalue_17
                                  (bind _returnvalue_18 (`ModAPI.WriteDataTableValue` _returnvalue _gridactors RowId "industrialLabor" (`KismetStringLibrary.Conv_BoolToString` GridActor_industrialLabor)))
                                  (if _returnvalue_18
                                    (bind _returnvalue_19 (`ModAPI.WriteDataTableValue` _returnvalue _gridactors RowId "maxAgents_contextual" (`KismetStringLibrary.Conv_IntToString` GridActor_maxAgents_contextual)))
                                    (if _returnvalue_19
                                      (bind _returnvalue_20 (`ModAPI.WriteDataTableValue` _returnvalue _gridactors RowId "decorType" (`KismetStringLibrary.Conv_NameToString` GridActor_decorType)))
                                      (if _returnvalue_20
                                        (bind _returnvalue_21 (`ModAPI.WriteDataTableValue` _returnvalue _gridactors RowId "toolbarGroup" (`KismetStringLibrary.Conv_NameToString` GridActor_toolbarGroup)))
                                        (if _returnvalue_21
                                          (bind _returnvalue_22 (`ModAPI.WriteDataTableValue` _returnvalue _gridactors RowId "toolbarGroupSort" (`KismetStringLibrary.Conv_IntToString` GridActor_toolbarGroupSort)))
                                          (if _returnvalue_22
                                            (bind _returnvalue_23 (`ModAPI.WriteDataTableValue` _returnvalue _gridactors RowId "structureType" (`KismetStringLibrary.Conv_NameToString` GridActor_structureType)))
                                            (if _returnvalue_23
                                              (bind _returnvalue_24 (`ModAPI.WriteDataTableValue` _returnvalue _gridactors RowId "randomlyRotate" (`KismetStringLibrary.Conv_BoolToString` GridActor_randomlyRotate)))
                                              (if _returnvalue_24
                                                (bind _returnvalue_25 (`ModAPI.WriteDataTableValue` _returnvalue _gridactors RowId "refundRule" (`KismetStringLibrary.Conv_NameToString` GridActor_refundRule)))
                                                (if _returnvalue_25
                                                  (bind _returnvalue_26 (`ModAPI.WriteDataTableValue` _returnvalue _gridactors RowId "Quality" (`KismetStringLibrary.Conv_IntToString` GridActor_Quality)))
                                                  (if _returnvalue_26
                                                    (bind _returnvalue_27 (`ModAPI.WriteDataTableValue` _returnvalue _gridactors RowId "TooltipTags" (`self.Convert AName to Stringified Value` GridActor_TooltipTags)))
                                                    (if _returnvalue_27
                                                      (bind _returnvalue_28 (`ModAPI.WriteDataTableValue` _returnvalue _gridactors RowId "constructionTime" (`KismetStringLibrary.Conv_DoubleToString` GridActor_constructionTime)))
                                                      (if _returnvalue_28
                                                        (bind _returnvalue_29 (`ModAPI.WriteDataTableValue` _returnvalue _gridactors RowId "useCustomIcon" (`KismetStringLibrary.Conv_BoolToString` GridActor_useCustomIcon)))
                                                        (if _returnvalue_29
                                                          (bind _returnvalue_30 (`ModAPI.WriteDataTableValue` _returnvalue _gridactors RowId "Icon" (`self.Construct Icon Ref` GridActor_Icon)))
                                                          (if _returnvalue_30
                                                            (bind _returnvalue_31 (`ModAPI.WriteDataTableValue` _returnvalue _gridactors RowId "unlockPrerequisite" (`KismetStringLibrary.Conv_NameToString` GridActor_unlockPrerequisite)))
                                                            (if _returnvalue_31
                                                              (bind _returnvalue_32 (`ModAPI.WriteDataTableValue` _returnvalue _gridactors RowId "detailCue" (`KismetSystemLibrary.GetDisplayName` GridActor_detailCue)))
                                                              (if _returnvalue_32
                                                                (if (not true)
                                                                  (`self.Log Message` "failed to write to slot decorative"))
                                                                (else
                                                                  (`self.Log Message` "failed to write to slot decorative")))
                                                              (else
                                                                (`self.Log Message` "failed to write to slot decorative")))
                                                            (else
                                                              (`self.Log Message` "failed to write to slot decorative")))
                                                          (else
                                                            (`self.Log Message` "failed to write to slot decorative")))
                                                        (else
                                                          (`self.Log Message` "failed to write to slot decorative")))
                                                      (else
                                                        (`self.Log Message` "failed to write to slot decorative")))
                                                    (else
                                                      (`self.Log Message` "failed to write to slot decorative")))
                                                  (else
                                                    (`self.Log Message` "failed to write to slot decorative")))
                                                (else
                                                  (`self.Log Message` "failed to write to slot decorative")))
                                              (else
                                                (`self.Log Message` "failed to write to slot decorative")))
                                            (else
                                              (`self.Log Message` "failed to write to slot decorative")))
                                          (else
                                            (`self.Log Message` "failed to write to slot decorative")))
                                        (else
                                          (`self.Log Message` "failed to write to slot decorative")))
                                      (else
                                        (`self.Log Message` "failed to write to slot decorative")))
                                    (else
                                      (`self.Log Message` "failed to write to slot decorative")))
                                  (else
                                    (`self.Log Message` "failed to write to slot decorative")))
                                (else
                                  (`self.Log Message` "failed to write to slot decorative")))
                              (else
                                (`self.Log Message` "failed to write to slot decorative")))
                            (else
                              (`self.Log Message` "failed to write to slot decorative")))
                          (else
                            (`self.Log Message` "failed to write to slot decorative")))
                        (else
                          (`self.Log Message` "failed to write to slot decorative")))
                      (else
                        (`self.Log Message` "failed to write to slot decorative")))
                    (else
                      (`self.Log Message` "failed to write to slot decorative")))
                  (else
                    (`self.Log Message` "failed to write to slot decorative")))
                (else
                  (`self.Log Message` "failed to write to slot decorative")))
              (else
                (`self.Log Message` "failed to write to slot decorative")))
            (else
              (`self.Log Message` "failed to write to slot decorative")))
          (else
            (`self.Log Message` "failed to write to slot decorative")))
        (else
          (`self.Log Message` "failed to write to slot decorative")))
      (else
        (`self.Log Message` "failed to write to slot decorative")))
    (else
      (`self.Log Message` "failed to add slot deco DT row"))))

(fn `Write Icons Row`
  (params (Icon :type "IconDataRowBase Structure") (`Row Id` :type Name))
  (locals (Icons_Buildings :type Name :default "BuildingIcons"))
  (bind _returnvalue (`ModAPI.GetModAPI`))
  (bind _icons_buildings (`local.Icons_Buildings`))
  (`ModAPI.AddDataTable` _returnvalue _icons_buildings null)
  (bind _returnvalue_2 (`ModAPI.AddDataTableRow` _returnvalue _icons_buildings `Row Id`))
  (if _returnvalue_2
    (bind _returnvalue_3 (`ModAPI.WriteDataTableValue` _returnvalue _icons_buildings `Row Id` "Icon" (`self.Construct Icon Ref` Icon_Icon)))
    (if (not _returnvalue_3)
      (`self.Log Message` "failed to add icon to Icons_Buildings row"))
    (else
      (`self.Log Message` "failed to add row to Icons_Buildings DT"))))

(fn `Write SlotDecoratives Row`
  (params (RowId :type Name) (SlotDecorative :type "SlotDecorative Structure"))
  (locals (SlotDecoratives :type Name :default "SlotDecoratives"))
  (bind _returnvalue (`ModAPI.GetModAPI`))
  (bind _returnvalue_2 (`ModAPI.AddDataTableRow` _returnvalue (`local.SlotDecoratives`) RowId))
  (if _returnvalue_2
    (bind _returnvalue_3 (`ModAPI.WriteDataTableValue` _returnvalue (`local.SlotDecoratives`) RowId "LocKey" SlotDecorative_LocKey))
    (if _returnvalue_3
      (bind _returnvalue_4 (`ModAPI.WriteDataTableValue` _returnvalue (`local.SlotDecoratives`) RowId "decorativeActor" (`self.Construct BP Ref` SlotDecorative_decorativeActor)))
      (if _returnvalue_4
        (bind _returnvalue_5 (`ModAPI.WriteDataTableValue` _returnvalue (`local.SlotDecoratives`) RowId "desiredSubSlot" (`|GetEnumeratorNameAsString` SlotDecorative_desiredSubSlot)))
        (if _returnvalue_5
          (bind _returnvalue_6 (`ModAPI.WriteDataTableValue` _returnvalue (`local.SlotDecoratives`) RowId "pathingEffect" (`|GetEnumeratorNameAsString` SlotDecorative_pathingEffect)))
          (if (not _returnvalue_6)
            (`self.Log Message` "failed to write to slot decorative"))
          (else
            (`self.Log Message` "failed to write to slot decorative")))
        (else
          (`self.Log Message` "failed to write to slot decorative")))
      (else
        (`self.Log Message` "failed to write to slot decorative")))
    (else
      (`self.Log Message` "failed to add slot deco DT row"))))

(fn `Write Strings Row`
  (params (Value :type String) (`Row Id` :type Name))
  (locals (StringsDT :type Name :default "Strings"))
  (bind _returnvalue (`ModAPI.GetModAPI`))
  (bind _stringsdt (`local.StringsDT`))
  (bind _returnvalue_2 (`ModAPI.AddDataTableRow` _returnvalue _stringsdt `Row Id`))
  (if _returnvalue_2
    (bind _returnvalue_3 (`ModAPI.WriteDataTableValue` _returnvalue _stringsdt `Row Id` "Value" Value))
    (if (not _returnvalue_3)
      (`self.Log Message` "failed to write strings DT \"Value\""))
    (else
      (`self.Log Message` "failed to add strings DT row"))))