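; Decorative gravel floor actor that scatters a random number of small grass instances over its Cube mesh.
; The Construction Script clears GrassHISM01 and refills it with local-space instances at random XY points within the Cube's bounds, at a fixed height with random yaw and scale.
; Placement is unseeded, so it changes on each construction.
; An unconnected variant using Min/MaxGrasstoSpawn never runs, and the Event Graph is empty.
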(fn `UserConstructionScript`
  (locals (NewLocalVar :type Integer :default 0))
  (bind _returnvalue (`KismetMathLibrary.RandomFloatInRange` 0.05 0.1))
  (bind (_origin _boxextent) (`KismetSystemLibrary.GetComponentBounds` (`self.Cube`)))
  (bind _returnvalue_2 (+ (.z _boxextent) (.z _origin)))
  (`InstancedStaticMeshComponent.ClearInstances` (`self.GrassHISM_01`))
  (for _ (range (+ (`KismetMathLibrary.RandomIntegerInRange` 0 50) 1))
    (`InstancedStaticMeshComponent.AddInstance` (`self.GrassHISM_01`) (`KismetMathLibrary.MakeTransform` (`KismetMathLibrary.MakeVector` (.x (`KismetMathLibrary.RandomPointInBoundingBox` (`KismetMathLibrary.MakeVector` 0.0 0.0 _returnvalue_2) (`KismetMathLibrary.MakeVector` (.x _boxextent) (.y _boxextent) _returnvalue_2))) (.y (`KismetMathLibrary.RandomPointInBoundingBox` (`KismetMathLibrary.MakeVector` 0.0 0.0 _returnvalue_2) (`KismetMathLibrary.MakeVector` (.x _boxextent) (.y _boxextent) _returnvalue_2))) 2.0) (`KismetMathLibrary.MakeRotator` 0.0 0.0 (`KismetMathLibrary.RandomFloatInRange` 0.0 360.0)) (`KismetMathLibrary.MakeVector` _returnvalue _returnvalue _returnvalue)) false)))