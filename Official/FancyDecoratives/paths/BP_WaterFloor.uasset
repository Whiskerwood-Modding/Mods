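; BP_WaterFloor is a decorative water tile that fits its depth to whatever lies beneath it.
; ActualiserVolume runs at construction and shortly after BeginPlay, box-tracing downward on the Camera channel.
; On a hit, it moves WaterGround to the bottom, centers and stretches WaterVolume over the gap, then passes the hit distance to dynamic water materials on the volume and surface.
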(event `self.ReceiveBeginPlay`
  (`KismetSystemLibrary.Delay` 0.2)
  (`self.ActualiserVolume`))

(fn `ActualiserVolume`
  (bind _x (.x (`self.K2_GetActorLocation`)))
  (bind _y (.y (`self.K2_GetActorLocation`)))
  (`PrimitiveComponent.SetMaterial` (`self.WaterVolume`) 0 "/Game/Mods/FancyDecoratives/others/MI_WaterFancy_Inst.MI_WaterFancy_Inst")
  (bind (_outhit _returnvalue) (`KismetSystemLibrary.BoxTraceSingle` :`Start` (`KismetMathLibrary.MakeVector` _x _y (+ (.z (`self.K2_GetActorLocation`)) 0.0)) :`End` (`KismetMathLibrary.MakeVector` _x _y -5000.0) :`HalfSize` (15.0 15.0 1.0) :`TraceChannel` "TraceTypeQuery2" :`bTraceComplex` true :`DrawDebugType` "ForDuration"))
  (if _returnvalue
    (bind (_bblockinghit _binitialoverlap _time _distance) (`GameplayStatics.BreakHitResult` _outhit))
    (`SceneComponent.K2_SetRelativeLocation` (`self.WaterGround`) (`KismetMathLibrary.MakeVector` 0.0 0.0 (* (+ _distance -1.0) -1.0)) false false)
    (`SceneComponent.K2_SetRelativeLocation` (`self.WaterVolume`) (`KismetMathLibrary.MakeVector` 0.0 0.0 (+ (* (/ _distance 2.0) -1.0) 7.5)) false false)
    (`SceneComponent.SetRelativeScale3D` (`self.WaterVolume`) (`KismetMathLibrary.MakeVector` 0.195 0.195 (+ (* _distance (/ 0.1365 35.0)) 0.06)))
    (bind _returnvalue_2 (`PrimitiveComponent.CreateDynamicMaterialInstance` (`self.WaterVolume`) 0 "/Game/Mods/FancyDecoratives/others/MI_WaterFancy_Inst.MI_WaterFancy_Inst" "None"))
    (bind _output_get (set `self.myWaterMaterial` _returnvalue_2))
    (`MaterialInstanceDynamic.SetScalarParameterValue` _output_get "Distance" _distance)
    (bind _returnvalue_3 (`PrimitiveComponent.CreateDynamicMaterialInstance` (`self.WaterSurface`) 0 "/Game/Mods/FancyDecoratives/others/MI_WaterFancy_Inst.MI_WaterFancy_Inst" "None"))
    (bind _output_get_2 (set `self.myWaterMaterial` _returnvalue_3))
    (`MaterialInstanceDynamic.SetScalarParameterValue` _output_get_2 "Distance" _distance)))

(fn `UserConstructionScript`
  (`self.ActualiserVolume`))