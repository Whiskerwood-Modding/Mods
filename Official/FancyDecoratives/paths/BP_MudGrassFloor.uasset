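; Decorative mud-and-grass floor actor that procedurally scatters grass and rocks across its Cube mesh at construction, with no runtime logic.
; A coin flip adds either a few small rocks or one larger grass clump, and a random count of grass is split between two HISMs.
; Instances get random positions within the Cube bounds, yaw and scale, unseeded.
; Only the grass HISMs are cleared beforehand, not RockHISM.
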(fn `UserConstructionScript`
  (locals (NewLocalVar :type Integer :default 0))
  (bind _returnvalue (`KismetMathLibrary.RandomFloatInRange` 0.005 0.007))
  (bind _returnvalue_2 (`KismetMathLibrary.RandomFloatInRange` 0.15 0.25))
  (bind _returnvalue_3 (`KismetMathLibrary.RandomFloatInRange` 0.08 0.1))
  (bind _returnvalue_4 (`KismetMathLibrary.RandomFloatInRange` 0.05 0.1))
  (bind (_origin _boxextent) (`KismetSystemLibrary.GetComponentBounds` (`self.Cube`)))
  (bind (_origin_2 _boxextent_2) (`KismetSystemLibrary.GetComponentBounds` (`self.Cube`)))
  (bind (_origin_3 _boxextent_3) (`KismetSystemLibrary.GetComponentBounds` (`self.Cube`)))
  (bind (_origin_4 _boxextent_4) (`KismetSystemLibrary.GetComponentBounds` (`self.Cube`)))
  (bind _returnvalue_5 (+ (.z _boxextent_2) (.z _origin_2)))
  (bind _returnvalue_6 (+ (.z _boxextent_3) (.z _origin_3)))
  (bind _returnvalue_7 (+ (.z _boxextent_4) (.z _origin_4)))
  (bind _returnvalue_8 (+ (.z _boxextent) (.z _origin)))
  (set `self.GrassToSpawn` (`KismetMathLibrary.RandomIntegerInRange` (`self.minGrasstoSpawn`) (`self.maxGrasstoSpawn`)))
  (`InstancedStaticMeshComponent.ClearInstances` (`self.GrassHISM_01`))
  (`InstancedStaticMeshComponent.ClearInstances` (`self.GrassHISM_02`))
  (if (`KismetMathLibrary.Conv_IntToBool` (`KismetMathLibrary.RandomIntegerInRange` 0 1))
    (for _ (range (`KismetMathLibrary.RandomIntegerInRange` 0 6))
      (`InstancedStaticMeshComponent.AddInstance` (`self.RockHISM`) (`KismetMathLibrary.MakeTransform` (`KismetMathLibrary.MakeVector` (.x (`KismetMathLibrary.RandomPointInBoundingBox` (`KismetMathLibrary.MakeVector` 0.0 0.0 _returnvalue_8) (`KismetMathLibrary.MakeVector` (.x _boxextent) (.y _boxextent) _returnvalue_8))) (.y (`KismetMathLibrary.RandomPointInBoundingBox` (`KismetMathLibrary.MakeVector` 0.0 0.0 _returnvalue_8) (`KismetMathLibrary.MakeVector` (.x _boxextent) (.y _boxextent) _returnvalue_8))) 2.2) (`KismetMathLibrary.MakeRotator` 0.0 0.0 (`KismetMathLibrary.RandomFloatInRange` 0.0 360.0)) (`KismetMathLibrary.MakeVector` _returnvalue _returnvalue _returnvalue)) false)
      (for _ (range (`self.GrassToSpawn`)) :!label _label
        (if (`KismetMathLibrary.Conv_IntToBool` (`KismetMathLibrary.RandomIntegerInRange` 0 1))
          (`InstancedStaticMeshComponent.AddInstance` (`self.GrassHISM_01`) (`KismetMathLibrary.MakeTransform` (`KismetMathLibrary.MakeVector` (.x (`KismetMathLibrary.RandomPointInBoundingBox` (`KismetMathLibrary.MakeVector` 0.0 0.0 _returnvalue_7) (`KismetMathLibrary.MakeVector` (.x _boxextent_4) (.y _boxextent_4) _returnvalue_7))) (.y (`KismetMathLibrary.RandomPointInBoundingBox` (`KismetMathLibrary.MakeVector` 0.0 0.0 _returnvalue_7) (`KismetMathLibrary.MakeVector` (.x _boxextent_4) (.y _boxextent_4) _returnvalue_7))) 2.0) (`KismetMathLibrary.MakeRotator` 0.0 0.0 (`KismetMathLibrary.RandomFloatInRange` 0.0 360.0)) (`KismetMathLibrary.MakeVector` _returnvalue_4 _returnvalue_4 _returnvalue_4)) false)
          (else
            (`InstancedStaticMeshComponent.AddInstance` (`self.GrassHISM_02`) (`KismetMathLibrary.MakeTransform` (`KismetMathLibrary.MakeVector` (.x (`KismetMathLibrary.RandomPointInBoundingBox` (`KismetMathLibrary.MakeVector` 0.0 0.0 _returnvalue_6) (`KismetMathLibrary.MakeVector` (.x _boxextent_3) (.y _boxextent_3) _returnvalue_6))) (.y (`KismetMathLibrary.RandomPointInBoundingBox` (`KismetMathLibrary.MakeVector` 0.0 0.0 _returnvalue_6) (`KismetMathLibrary.MakeVector` (.x _boxextent_3) (.y _boxextent_3) _returnvalue_6))) 2.0) (`KismetMathLibrary.MakeRotator` 0.0 0.0 (`KismetMathLibrary.RandomFloatInRange` 0.0 360.0)) (`KismetMathLibrary.MakeVector` _returnvalue_3 _returnvalue_3 _returnvalue_3)) false)))))
    (else
      (`InstancedStaticMeshComponent.AddInstance` (`self.GrassHISM_02`) (`KismetMathLibrary.MakeTransform` (`KismetMathLibrary.MakeVector` (.x (`KismetMathLibrary.RandomPointInBoundingBox` (`KismetMathLibrary.MakeVector` 0.0 0.0 _returnvalue_5) (`KismetMathLibrary.MakeVector` (.x _boxextent_2) (.y _boxextent_2) _returnvalue_5))) (.y (`KismetMathLibrary.RandomPointInBoundingBox` (`KismetMathLibrary.MakeVector` 0.0 0.0 _returnvalue_5) (`KismetMathLibrary.MakeVector` (.x _boxextent_2) (.y _boxextent_2) _returnvalue_5))) 2.0) (`KismetMathLibrary.MakeRotator` 0.0 0.0 (`KismetMathLibrary.RandomFloatInRange` 0.0 360.0)) (`KismetMathLibrary.MakeVector` _returnvalue_2 _returnvalue_2 _returnvalue_2)) false)))
  (goto _label))