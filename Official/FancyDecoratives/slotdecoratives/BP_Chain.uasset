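; BP_Chain is a decorative chain actor that builds itself along an editable spline.
; The construction script adds overlapping spline mesh links, spaced by mesh size minus overlap, skipping any that would run past the spline's end.
; Successive links alternate roll between 0 and 90 degrees to look interlocked, with tangent lengths clamped to the link spacing.
; The event graph holds only empty placeholder events.
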(fn `UserConstructionScript`
  (locals (NewLocalVar :type "Vector Structure" :default (0.0 90.0 0.0)))
  (bind _spline (`self.Spline`))
  (bind _meshsize (`self.MeshSize`))
  (bind _spline_2 (`self.Spline`))
  (for _index (range (+ (`KismetMathLibrary.FTrunc` (/ (`SplineComponent.GetSplineLength` (`self.Spline`)) (- (`self.MeshSize`) (`self.overlap`)))) 1))
    (bind _returnvalue (* _index (- _meshsize (`self.overlap`))))
    (bind _returnvalue_2 (+ _returnvalue _meshsize))
    (if (not (> _returnvalue_2 (`SplineComponent.GetSplineLength` (`self.Spline`))))
      (bind _returnvalue_3 (`AddComponent|NODE_AddSplineMeshComponent-1` :`bManualAttachment` true))
      (`SceneComponent.K2_AttachToComponent` _returnvalue_3 (`self.DefaultSceneRoot`) "None" "KeepRelative" "KeepRelative" "KeepRelative" true)
      (bind _returnvalue_4 (`KismetMathLibrary.SelectFloat` 0.0 90.0 (== (mod _index 2) 0)))
      (`SplineMeshComponent.SetStartRollDegrees` _returnvalue_3 _returnvalue_4 true)
      (`SplineMeshComponent.SetEndRollDegrees` _returnvalue_3 _returnvalue_4 true)
      (`SplineMeshComponent.SetStartAndEnd` _returnvalue_3 (`SplineComponent.GetLocationAtDistanceAlongSpline` _spline_2 _returnvalue "Local") (`KismetMathLibrary.ClampVectorSize` (`SplineComponent.GetTangentAtDistanceAlongSpline` _spline_2 _returnvalue "Local") 0.0 (- (`self.MeshSize`) (`self.overlap`))) (`SplineComponent.GetLocationAtDistanceAlongSpline` _spline _returnvalue_2 "Local") (`KismetMathLibrary.ClampVectorSize` (`SplineComponent.GetTangentAtDistanceAlongSpline` _spline _returnvalue_2 "Local") 0.0 (- (`self.MeshSize`) (`self.overlap`))) true))))