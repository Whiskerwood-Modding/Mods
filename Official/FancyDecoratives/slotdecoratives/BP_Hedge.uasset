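; Decorative hedge actor that procedurally builds a column of bush meshes in its construction script, with no runtime logic.
; Each of NombreDeCopies layers is raised by EspacementHauteur and holds two clusters of six bushes, offset along Y.
; AddBush creates each static mesh component from ListeMeshes with preset scales and mostly random rotations.
; The randomness is unseeded, so the hedge's look changes whenever construction reruns.
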(fn `add Bush`
  (params (Location :type "Vector Structure") (Rotation :type "Rotator Structure") (Scale :type "Vector Structure") (StaticMesh :type "StaticMesh Object Reference"))
  (bind _returnvalue (`AddComponent|NODE_AddStaticMeshComponent-2` :`RelativeTransform` (`KismetMathLibrary.MakeTransform` (0.0 0.0 0.0) Rotation Scale)))
  (`StaticMeshComponent.SetStaticMesh` _returnvalue StaticMesh)
  (`SceneComponent.K2_SetRelativeLocation` _returnvalue Location false false))

(fn `UserConstructionScript`
  (locals (NewLocalVar :type "Vector Structure" :default (0.0 90.0 0.0)))
  (bind _returnvalue (`KismetMathLibrary.RandomFloatInRange` -5.0 5.0))
  (bind _listemeshes (`self.ListeMeshes`))
  (bind _listemeshes_2 (`self.ListeMeshes`))
  (bind _returnvalue_2 (`KismetMathLibrary.MakeRotator` _returnvalue (`KismetMathLibrary.RandomFloatInRange` 310.0 380.0) _returnvalue))
  (for _index (range (`self.NombreDeCopies`))
    (bind _returnvalue_3 (`KismetMathLibrary.Conv_IntToDouble` (* _index (`self.EspacementHauteur`))))
    (bind _returnvalue_4 (`KismetMathLibrary.MakeVector` 0.0 0.0 _returnvalue_3))
    (`self.add Bush` _returnvalue_4 _returnvalue_2 (0.108 0.146 0.138) _listemeshes)
    (`self.add Bush` _returnvalue_4 _returnvalue_2 (0.108 0.146 0.138) _listemeshes)
    (`self.add Bush` _returnvalue_4 _returnvalue_2 (0.1276 0.1661 0.1576) _listemeshes)
    (`self.add Bush` _returnvalue_4 _returnvalue_2 (0.0893 0.1467 0.1478) _listemeshes)
    (`self.add Bush` _returnvalue_4 _returnvalue_2 (0.108 0.146 0.0936) _listemeshes)
    (`self.add Bush` _returnvalue_4 (struct :`Pitch` 554.6 :`Yaw` -19.4063 :`Roll` 5.316) (0.0893 0.14579 0.1478) _listemeshes)
    (bind _returnvalue_5 (`KismetMathLibrary.MakeVector` 0.0 25.0 _returnvalue_3))
    (`self.add Bush` _returnvalue_5 _returnvalue_2 (0.108 0.146 0.138) _listemeshes_2)
    (`self.add Bush` _returnvalue_5 _returnvalue_2 (0.108 0.146 0.138) _listemeshes_2)
    (`self.add Bush` _returnvalue_5 _returnvalue_2 (0.1276 0.1661 0.1576) _listemeshes_2)
    (`self.add Bush` _returnvalue_5 _returnvalue_2 (0.0893 0.1467 0.1478) _listemeshes_2)
    (`self.add Bush` _returnvalue_5 _returnvalue_2 (0.108 0.146 0.0936) _listemeshes_2)
    (`self.add Bush` _returnvalue_5 (struct :`Pitch` 554.6 :`Yaw` -19.4063 :`Roll` 5.316) (0.0893 0.14579 0.1478) _listemeshes_2)))