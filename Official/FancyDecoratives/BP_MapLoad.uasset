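; Map-load helper for the FancyDecoratives mod that triggers waterfall checks when a game loads or a building spawns.
; On BeginPlay it binds to the mod API's loading-finished and building-spawned events.
; After a short delay, it calls CheckUnder on every BP_WaterFall once loading finishes, logging each one, or on the spawned actor if it is a waterfall.
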(event `self.ReceiveBeginPlay`
  (add `ModAPI.onLoadingFinished` (`ModAPI.GetModAPI`) (delegate `OnLoadingFinished`))
  (add `ModAPI.onBuildingSpawned` (`ModAPI.GetModAPI`) (delegate `OnWaterfallSpawned`)))

(event `OnLoadingFinished`
  (`KismetSystemLibrary.Delay` 0.2)
  (bind _outactors (`GameplayStatics.GetAllActorsOfClass` "/Game/Mods/FancyDecoratives/decors/BP_WaterFall.BP_WaterFall_C"))
  (for _array_element _outactors
    (bind _asbp_water_fall (cast `/Game/Mods/FancyDecoratives/decors/BP_WaterFall` _array_element))
    (`ModAPI.LogMessage` (`ModAPI.GetModAPI`) "loading finished" true)
    (`/Game/Mods/FancyDecoratives/decors/BP_WaterFall.checkUnder` _asbp_water_fall)))

(event `OnWaterfallSpawned`
  (params (Actor :type "Actor Object Reference"))
  (`KismetSystemLibrary.Delay` 0.2)
  (bind _asbp_water_fall (cast `/Game/Mods/FancyDecoratives/decors/BP_WaterFall` Actor))
  (`/Game/Mods/FancyDecoratives/decors/BP_WaterFall.checkUnder` _asbp_water_fall))

(fn `UserConstructionScript`)