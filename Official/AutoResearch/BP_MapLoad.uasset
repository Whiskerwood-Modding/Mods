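; AutoResearch mod load Blueprint, an unfinished scaffold that currently performs no research automation.
; On BeginPlay it logs through the mod API and binds to loading finished, where it only fetches the Arco system.
; The research-finished handler logs the unlock ID, but its binding to the Holdings Relay is disconnected.
; Other unwired experiments probe tech tree widgets, lab components, tier resource slots and active research state.
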(event `self.ReceiveBeginPlay`
  (bind _returnvalue (`ModAPI.GetModAPI`))
  (`ModAPI.LogMessage` _returnvalue "AutoResearch loaded" true)
  (add `ModAPI.onLoadingFinished` _returnvalue (delegate `OnLoadingFinished`)))

(event `OnLoadingFinished`
  (bind (_out_isvalid _returnvalue) (`ArcoSystems.GetArcoSys`)))

(event `OnRunningChanged`
  (params (IsRunning :type Boolean)))

(event `OnResearchFinished`
  (params (unlockId :type Name))
  (`ModAPI.LogMessage` (`ModAPI.GetModAPI`) (`KismetStringLibrary.Conv_NameToString` unlockId) true))

(fn `UserConstructionScript`)