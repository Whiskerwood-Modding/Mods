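; Map-load mod Blueprint that injects a storage indicator widget into the game's UI directly after SeasonSummary.
; On BeginPlay it registers English and French title strings through the mod API, then after a short delay searches all UserWidgets for SeasonSummary by name.
; It re-adds that widget's VerticalBox siblings in order, inserting WBP_StorIndicator after SeasonSummary.
; The indicator's title uses the localized string, falling back to English when empty.
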(event `self.ReceiveBeginPlay`
  (bind _returnvalue (`LocManager.GetWordFromKey` (`Backbone.GetLocManager`) (`self.Lockey`)))
  (bind _storagetitle (`/Game/Mods/StorageIndicator/WBP_StorIndicator.StorageTitle` (`self.widget`)))
  (`ModAPI.AddNewStrings` (`ModAPI.GetModAPI`) "en" (`|MakeMap` (`self.Lockey`) (`self.englishString`)))
  (`ModAPI.AddNewStrings` (`ModAPI.GetModAPI`) "fr" (`|MakeMap` (`self.Lockey`) (`self.frenchString`)))
  (`KismetSystemLibrary.Delay` 0.2)
  (bind _foundwidgets (`WidgetBlueprintLibrary.GetAllWidgetsOfClass` "/Script/UMG.UserWidget" false))
  (for _array_element _foundwidgets
    (if (== (`KismetSystemLibrary.GetObjectName` _array_element) "SeasonSummary")
      (bind _returnvalue_2 (`Widget.GetParent` _array_element))
      (bind _asvertical_box (cast `VerticalBox` _returnvalue_2))
      (bind _returnvalue_3 (`PanelWidget.GetAllChildren` _returnvalue_2))
      (set `self.localobjects` _returnvalue_3)
      (`KismetArrayLibrary.Array_Clear` _returnvalue_3)
      (for _array_element_2 (`self.localobjects`)
        (if (== (`KismetSystemLibrary.GetObjectName` _array_element_2) "SeasonSummary")
          (`VerticalBox.AddChildToVerticalBox` _asvertical_box _array_element_2)
          (bind _returnvalue_4 (`|CreateWidget` "/Game/Mods/StorageIndicator/WBP_StorIndicator.WBP_StorIndicator_C" (`GameplayStatics.GetPlayerController` 0)))
          (bind _output_get (set `self.Widget` _returnvalue_4))
          (if (`KismetStringLibrary.IsEmpty` _returnvalue)
            (`TextBlock.SetText` _storagetitle (`KismetTextLibrary.Conv_StringToText` (`self.englishString`)))
            (else
              (`TextBlock.SetText` _storagetitle (`KismetTextLibrary.Conv_StringToText` _returnvalue))))
          (`VerticalBox.AddChildToVerticalBox` _asvertical_box _output_get)
          (else
            (`VerticalBox.AddChildToVerticalBox` _asvertical_box _array_element_2)))))))

(fn `UserConstructionScript`)