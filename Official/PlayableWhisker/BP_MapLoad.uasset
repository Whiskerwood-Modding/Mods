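; Map-load actor for the PlayableWhisker mod that lets F6 switch between the normal play pawn and a controllable BP_PlayableWhisker.
; Once loading finishes, it enables input and caches the PlayHud widget.
; Entering saves the camera state, spawns and possesses the Whisker at the cursor (with fallbacks) and hides the HUD.
; Exiting restores pawn, camera, HUD and input mode, then destroys the Whisker.
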(event `self.ReceiveBeginPlay`
  (add `ModAPI.onLoadingFinished` (`ModAPI.GetModAPI`) (delegate `OnLoadingFinished`)))

(event `OnLoadingFinished`
  (`self.EnableInput` (`GameplayStatics.GetPlayerController` 0))
  (bind _foundwidgets (`WidgetBlueprintLibrary.GetAllWidgetsOfClass` "/Script/ProjectArco.PlayHud"))
  (for _array_element _foundwidgets
    (set `self.PlayerHud` _array_element)))

(event `Key|F6`
  (params (Key :type "Key Structure"))
  (bind _returnvalue (`GameplayStatics.GetPlayerController` 0))
  (bind _returnvalue_2 (`GameplayStatics.GetPlayerController` 0))
  (bind _playerhud (`self.PlayerHud`))
  (:`Pressed`
    (if (`self.IsInWhiskerMode`)
      (bind _asbp_pawn_play (cast `/Game/Code/UnrealComponents/BP_Pawn_Play` (`self.OriginalViewTarget`)))
      (`Controller.Possess` _returnvalue_2 _asbp_pawn_play)
      (set `Pawn_Play.m_desiredPanPos` (`self.OriginalViewPos`) _asbp_pawn_play)
      (set `Pawn_Play.m_desiredRot` (`self.OriginalViewRot`) _asbp_pawn_play)
      (set `Pawn_Play.m_desiredZoomDist` (`self.OriginalViewZoom`) _asbp_pawn_play)
      (`PlayerController.SetViewTargetWithBlend` _returnvalue_2 (`self.OriginalViewTarget`) 1.0 "VTBlend_Linear" 0.0 false)
      (`self.Log` "Destroying")
      (`self.K2_DestroyActor` (`self.PlayableWhisker`))
      (`self.Log` "Adding playhud back to viewport")
      (`UserWidget.AddToViewport` _playerhud 1)
      (`self.Log` "Setting input mode to game and UI")
      (`WidgetBlueprintLibrary.SetInputMode_GameAndUIEx` _returnvalue_2 _playerhud)
      (set `PlayerController.bShowMouseCursor` true _returnvalue_2)
      (set `self.IsInWhiskerMode` false)
      (`self.Log` "Done")
      (else
        (bind _output_get (set `self.OriginalViewTarget` (`Controller.GetViewTarget` (`GameplayStatics.GetPlayerController` 0))))
        (bind _asbp_pawn_play_2 (cast `/Game/Code/UnrealComponents/BP_Pawn_Play` _output_get))
        (set `self.OriginalViewPos` (`Pawn_Play.m_desiredPanPos` _asbp_pawn_play_2))
        (set `self.OriginalViewRot` (`Pawn_Play.m_desiredRot` _asbp_pawn_play_2))
        (set `self.OriginalViewZoom` (`Pawn_Play.m_desiredZoomDist` _asbp_pawn_play_2))
        (bind _pos (`self.Get Spawn Pos`))
        (`self.Log` (`KismetStringLibrary.Concat_StrStr` (`KismetStringLibrary.Conv_VectorToString` (.location _pos)) (`KismetStringLibrary.Conv_RotatorToString` (.rotation _pos))))
        (bind _returnvalue_3 (`|SpawnActorFromClass` "/Game/Mods/PlayableWhisker/BP_PlayableWhisker.BP_PlayableWhisker_C" (`KismetMathLibrary.MakeTransform` (.location _pos) (.rotation _pos)) "Undefined" "MultiplyWithRoot" null null))
        (bind _output_get_2 (set `self.PlayableWhisker` _returnvalue_3))
        (`WidgetBlueprintLibrary.SetInputMode_GameOnly` _returnvalue)
        (`Controller.Possess` _returnvalue _output_get_2)
        (set `PlayerController.bShowMouseCursor` false _returnvalue)
        (set `self.IsInWhiskerMode` true)
        (`Widget.RemoveFromParent` (`self.PlayerHud`))
        (`self.Log` "Done")))))

(event `Key|Escape`
  (params (Key :type "Key Structure")))

(event `InputAction|pausemenu`
  (params (Key :type "Key Structure")))

(fn `Get Spawn Pos`
  (returns (Pos :type "Transform Structure"))
  (bind _returnvalue (`GameplayStatics.GetActorOfClass` "/Game/Code/UnrealComponents/BP_PlayerController_Play.BP_PlayerController_Play_C"))
  (`/Engine/EditorBlueprintResources/StandardMacros.IsValid` _returnvalue
    (:`Is Valid`
      (return (`KismetMathLibrary.MakeTransform` (`.worldPos_atZLevel` (break `CursorCastInfo` (break `ArcoPlayerState` (`PlayerController_Play.m_state` _returnvalue)))))))
    (:`Is Not Valid`
      (bind _returnvalue_2 (`GameplayStatics.GetActorOfClass` "/Game/Code/PlayerTools/BP_SelectTool.BP_SelectTool_C"))
      (bind _m_gridactoratgridpos (`SelectTool.m_gridActorAtGridPos` _returnvalue_2))
      (`/Engine/EditorBlueprintResources/StandardMacros.IsValid` _m_gridactoratgridpos
        (:`Is Valid`
          (return (`self.GetTransform` _m_gridactoratgridpos)))
        (:`Is Not Valid`
          (bind _returnvalue_3 (`GameplayStatics.GetActorOfClass` "/Script/ProjectArco.Prototype_Agent"))
          (`/Engine/EditorBlueprintResources/StandardMacros.IsValid` _returnvalue_3
            (:`Is Valid`
              (return (`self.GetTransform` _returnvalue_3)))
            (:`Is Not Valid`
              (`self.Log` "everything is invalid, falling back to 0,0,0")
              (return (`KismetMathLibrary.MakeTransform` (0.0 0.0 0.0))))))))))

(fn `Get Terrain Info`
  (bind (_out_isvalid _returnvalue) (`ArcoSystems.GetArcoSys`))
  (bind (_m_terrain_origin _m_terrain_extent _m_terrain_cells) (break `TiledTerrainData` (`ArcoSystems.m_terrain` _returnvalue)))
  (for (_array_element _array_index) _m_terrain_cells
    (if (> _array_index 100)
      (break)
      (else
        (`self.Log` (`KismetStringLibrary.Concat_StrStr` (`KismetStringLibrary.Conv_IntToString` (`KismetMathLibrary.Conv_ByteToInt` (`.Rocks` (break `TerrainCell` _array_element))))))))))

(fn `Log`
  (params (Msg :type String))
  (if (`self.LoggingOn?`)
    (`ModAPI.LogMessage` (`ModAPI.GetModAPI`) (`KismetStringLibrary.Concat_StrStr` "[PlayableWhisker] " Msg) true)))

(fn `UserConstructionScript`)