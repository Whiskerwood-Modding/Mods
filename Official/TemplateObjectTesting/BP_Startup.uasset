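; Startup Blueprint for the TemplateObjectTesting mod, which tests editing class default objects at runtime.
; On BeginPlay it loads the OreDistributorConfig_BP CDO through the mod API and marks it for retained editing.
; It overrides the config's non-ore yield, then loops over the ores, setting each yield by reference and logging the prior yield and name.
; An unconnected branch chain sketches per-ore-name edits but never runs.
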(event `self.ReceiveBeginPlay`
  (bind _returnvalue (`ModAPI.GetModAPI`))
  (bind _returnvalue_2 (`ModAPI.GetModAPI`))
  (bind _returnvalue_3 (`ModAPI.LoadCdoOfClass` _returnvalue_2 "/Game/Code/Systems/OreDistributorConfig_BP.OreDistributorConfig_BP_C"))
  (`ModAPI.MarkObjectTemplateForRetainedEditing` _returnvalue_2 _returnvalue_3)
  (bind _asore_distributor_config_bp (cast `/Game/Code/Systems/OreDistributorConfig_BP` _returnvalue_3))
  (bind _config (`OreDistributorConfigMule.config` _asore_distributor_config_bp))
  (setmembers `OreDistributorConfig` :`StructRef` _config :`NonOreYield` 5)
  (for _array_element (`.Ores` (break `OreDistributorConfig` _config))
    (bind (_name _yield) (break `OreDistributorOre` _array_element))
    (`ModAPI.LogMessage` _returnvalue (`KismetStringLibrary.Conv_IntToString` _yield) true)
    (`|VariableSetRef` _yield 20)
    (`ModAPI.LogMessage` _returnvalue (`KismetStringLibrary.Conv_NameToString` _name) true)))

(fn `UserConstructionScript`)