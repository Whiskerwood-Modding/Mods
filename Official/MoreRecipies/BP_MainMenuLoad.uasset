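; Main-menu load Blueprint for the MoreRecipies mod that adds a wood charcoal recipe through the game's mod API.
; On BeginPlay it registers the IndustryRecipes and TechUnlocksV2 tables, then writes the recipe row from a column-to-string map, logging failed writes.
; The tech-unlock creation, charcoal furnace child link and table dump are disconnected, and the option-changed handler is empty.
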(event `self.ReceiveBeginPlay`
  (add `ModAPI.onOptionChanged` (`ModAPI.GetModAPI`) (`|CreateDelegate` :!event `OnOptionChanged`))
  (`self.Init DTs`)
  (`self.Create New Row` "IndustryRecipes" "recipe.charcoal" (`self.WoodCharcoalRecipe`)))

(event `OnOptionChanged`
  (params (optionId :type String) (Value :type String)))

(fn `Create New Row`
  (params (DT :type Name) (Key :type Name) (Entries :type "Map of Name to String"))
  (`ModAPI.AddDataTableRow` (`ModAPI.GetModAPI`) DT Key)
  (bind (_keypin _valuepin) (`|MapForEach` Entries)
    (:`then`
      (bind _returnvalue (`ModAPI.WriteDataTableValue` (`ModAPI.GetModAPI`) DT Key _keypin _valuepin))
      (if (not _returnvalue)
        (`self.Log` (`KismetStringLibrary.Concat_StrStr` "Failed to write value to IndustryRecipes. Row: " (`KismetStringLibrary.Conv_NameToString` Key) " Column: " (`KismetStringLibrary.Conv_NameToString` _keypin) " Value: "))))))

(fn `Create New Unlock`
  (params (Key :type Name))
  (locals (`Row Id` :type Name))
  (bind _returnvalue (`ModAPI.GetModAPI`))
  (bind _returnvalue_2 (`ModAPI.GetModAPI`))
  (bind _returnvalue_3 (`ModAPI.GetModAPI`))
  (bind _row_id (`local.Row Id`))
  (bind _row_id_2 (`local.Row Id`))
  (bind _output_get (set `local.Row Id` Key))
  (`ModAPI.AddDataTableRow` _returnvalue_3 "TechUnlocksV2" _output_get)
  (`ModAPI.WriteDataTableValue` _returnvalue_3 "TechUnlocksV2" _row_id "useGridActorForLoc" "False")
  (`ModAPI.WriteDataTableValue` _returnvalue "TechUnlocksV2" _row_id "faction" "home")
  (`ModAPI.WriteDataTableValue` _returnvalue "TechUnlocksV2" (`local.Row Id`) "subCategory" "techCategory.Production")
  (`ModAPI.WriteDataTableValue` _returnvalue "TechUnlocksV2" _row_id_2 "associatedGridActor" "charcoalfurnace")
  (`ModAPI.WriteDataTableValue` _returnvalue_2 "TechUnlocksV2" _row_id_2 "associatedRecipe" "recipe.charcoal")
  (`ModAPI.WriteDataTableValue` _returnvalue_2 "TechUnlocksV2" _row_id_2 "researchable" "true")
  (`ModAPI.WriteDataTableValue` _returnvalue_2 "TechUnlocksV2" _row_id_2 "scienceCost" "20")
  (`ModAPI.WriteDataTableValue` _returnvalue_2 "TechUnlocksV2" _row_id_2 "researchTier" "0")
  (`ModAPI.WriteDataTableValue` _returnvalue_2 "TechUnlocksV2" _row_id_2 "prerequisiteUnlocks" "(\"unlock.charcoalfurnace\")")
  (`ModAPI.WriteDataTableValue` _returnvalue_2 "TechUnlocksV2" (`local.Row Id`) "tierSortOrder" "15"))

(fn `Init DTs`
  (bind _returnvalue (`ModAPI.GetModAPI`))
  (`ModAPI.AddDataTable` _returnvalue "IndustryRecipes" "/Game/Data/AssetLookups/IndustryRecipies.IndustryRecipies")
  (`ModAPI.AddDataTable` _returnvalue "TechUnlocksV2" "/Game/Data/AssetLookups/TechUnlocksV2.TechUnlocksV2"))

(fn `Log`
  (params (Message :type String))
  (if (`self.Log Messages?`)
    (`ModAPI.LogMessage` (`ModAPI.GetModAPI`) (`KismetStringLibrary.Concat_StrStr` "[" (`self.Mod Name`) "] " Message) true)))

(fn `UserConstructionScript`)