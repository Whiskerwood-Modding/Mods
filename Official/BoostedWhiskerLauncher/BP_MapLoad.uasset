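; BP_MapLoad is the Boosted Whisker Launcher mod's map actor, overriding the maximum horizontal and vertical distance of jump pads.
; On BeginPlay it binds to mod API events for option changes, loading completion and building spawns.
; Loading reads both saved options, with fallbacks, and option changes update the cached values; both then reapply them to every JumpPad, while newly spawned pads receive them individually.
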(event `self.ReceiveBeginPlay`
  (add `ModAPI.onOptionChanged` (`ModAPI.GetModAPI`) (`|CreateDelegate` :!event `OnOptionChanged`))
  (add `ModAPI.onLoadingFinished` (`ModAPI.GetModAPI`) (`|CreateDelegate` :!event `OnLoadingFinished`))
  (add `ModAPI.onBuildingSpawned` (`ModAPI.GetModAPI`) (`|CreateDelegate` :!event `onBuildingSpawned_Event`)))

(event `OnLoadingFinished`
  (bind _returnvalue (`ModAPI.ReadModOptionValue` (`ModAPI.GetModAPI`) (`self.MaxDistanceOptionId`) "5"))
  (`self.OnDistanceOptionChange` _returnvalue)
  (bind _returnvalue_2 (`ModAPI.ReadModOptionValue` (`ModAPI.GetModAPI`) (`self.MaxHeightOptionId`) "10"))
  (`self.OnHeightOptionChange` _returnvalue_2)
  (`self.SetAllJumpPads`))

(event `onBuildingSpawned_Event`
  (params (Actor :type "Actor Object Reference"))
  (bind _asjump_pad (cast `/Game/GridActors/JumpPad` Actor))
  (bind _jumppad (`/Game/GridActors/JumpPad.JumpPad` _asjump_pad))
  (set `JumpPad.maxHorizDistance` (`self.LocalMaxHorizonDistance`) _jumppad)
  (set `JumpPad.maxZDistance` (`self.LocalMaxHeight`) _jumppad))

(event `OnOptionChanged`
  (params (`option Id` :type String) (Value :type String))
  (`|ExecutionSequence`
    (:`then_0`
      (if (`KismetStringLibrary.EqualEqual_StrStr` `option Id` (`self.MaxDistanceOptionId`))
        (`self.Log Message` (`KismetStringLibrary.Concat_StrStr` "Old Distance: " (`KismetStringLibrary.Conv_IntToString` (`self.LocalMaxHorizonDistance`))) "BoostedLauncher")
        (`self.OnDistanceOptionChange` Value)
        (`self.SetAllJumpPads`)))
    (:`then_1`
      (if (`KismetStringLibrary.EqualEqual_StrStr` `option Id` (`self.MaxHeightOptionId`))
        (`self.Log Message` (`KismetStringLibrary.Concat_StrStr` "Old Height: " (`KismetStringLibrary.Conv_IntToString` (`self.LocalMaxHeight`))) "BoostedLauncher")
        (`self.OnHeightOptionChange` Value)
        (`self.SetAllJumpPads`)))))

(fn `Log Message`
  (params (Message :type String) (`Mod Name` :type String))
  (bind (_year _month _day _hour _minute _second _millisecond) (`KismetMathLibrary.BreakDateTime` (`KismetMathLibrary.Now`)))
  (`ModAPI.LogMessage` (`ModAPI.GetModAPI`) (`KismetStringLibrary.Concat_StrStr` "[" (`KismetStringLibrary.Conv_IntToString` _year) "-" (`KismetStringLibrary.Conv_IntToString` _month) "-" (`KismetStringLibrary.Conv_IntToString` _day) " " (`KismetStringLibrary.Conv_IntToString` _hour) ":" (`KismetStringLibrary.Conv_IntToString` _minute) ":" (`KismetStringLibrary.Conv_IntToString` _second) "." (`KismetStringLibrary.Conv_IntToString` _millisecond) "] [" `Mod Name` "]" Message)))

(fn `OnDistanceOptionChange`
  (params (Option :type String))
  (bind _output_get (set `self.LocalMaxHorizonDistance` (`KismetStringLibrary.Conv_StringToInt` Option)))
  (`self.Log Message` (`KismetStringLibrary.Concat_StrStr` "ValueChanged for Distance: " (`KismetStringLibrary.Conv_IntToString` _output_get)) (`self.MaxDistanceOptionId`)))

(fn `OnHeightOptionChange`
  (params (Option :type String))
  (bind _output_get (set `self.LocalMaxHeight` (`KismetStringLibrary.Conv_StringToInt` Option)))
  (`self.Log Message` (`KismetStringLibrary.Concat_StrStr` "ValueChanged for Height: " (`KismetStringLibrary.Conv_IntToString` _output_get)) (`self.MaxHeightOptionId`)))

(fn `SetAllJumpPads`
  (bind _outactors (`GameplayStatics.GetAllActorsOfClass` "/Game/GridActors/JumpPad.JumpPad_C"))
  (for _array_element _outactors
    (bind _jumppad (`/Game/GridActors/JumpPad.JumpPad` _array_element))
    (set `JumpPad.maxHorizDistance` (`self.LocalMaxHorizonDistance`) _jumppad)
    (set `JumpPad.maxZDistance` (`self.LocalMaxHeight`) _jumppad))
  (`self.Log Message` "=====Completed=====" "BoostedWhiskerLauncher"))

(fn `UserConstructionScript`)