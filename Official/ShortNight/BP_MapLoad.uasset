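; ShortNight mod map-load Blueprint that shortens nights by changing global time dilation.
; Tick polls WorldTime_BP for phase changes, saving the clamped game speed and applying the night multiplier at LATE NIGHT, then restoring it at MID DAY.
; The multiplier is parsed from a mod option string and follows option changes through a ModAPI binding.
; During night it reapplies the multiplier on Tick, overriding player speed changes.
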(event `self.ReceiveBeginPlay`
  (add `ModAPI.onOptionChanged` (`ModAPI.GetModAPI`) (`|CreateDelegate` :!event `OnOptionChanged`)))

(event `self.ReceiveTick`
  (params (DeltaSeconds :type "Float (single-precision)"))
  (bind _returnvalue (`GameplayStatics.GetActorOfClass` "/Game/Code/Systems/WorldTime_BP.WorldTime_BP_C"))
  (`/Engine/EditorBlueprintResources/StandardMacros.IsValid` _returnvalue
    (:`Is Valid`
      (bind _m_currentphase (`WorldTime.m_currentPhase` _returnvalue))
      (if (`|EnumInequality` _m_currentphase (`self.PreviousPhase`))
        (bind _output_get (set `self.PreviousPhase` _m_currentphase))
        (switch `EDayPhase` _output_get
          (:`MID_DAY`
            (`GameplayStatics.SetGlobalTimeDilation` (`self.PreviousTimeDilation`))
            (set `self.IsNight?` false))
          (:`LATE_NIGHT`
            (set `self.PreviousTimeDilation` (`KismetMathLibrary.FClamp` (`GameplayStatics.GetGlobalTimeDilation`) 0.5 20.0))
            (bind _returnvalue_2 (`ModAPI.ReadModOptionValue` (`ModAPI.GetModAPI`) (`self.NightLengthOptionId`) "5x"))
            (bind _dilation (`self.Set Dilation From Option` _returnvalue_2))
            (`GameplayStatics.SetGlobalTimeDilation` _dilation)
            (set `self.IsNight?` true)))
        (else
          ; Handle case that player changes game speed at night time
          (if (`self.IsNight?`)
            (`GameplayStatics.SetGlobalTimeDilation` (`self.SetTimeDilation`))))))))

(event `OnOptionChanged`
  (params (optionId :type String) (Value :type String))
  (if (`KismetStringLibrary.EqualEqual_StrStr` optionId (`self.NightLengthOptionId`))
    (`self.Set Dilation From Option` Value)))

(fn `Debug`)

(fn `Log Message`
  (params (Message :type String) (`Mod Name` :type String))
  (bind (_year _month _day _hour _minute _second _millisecond) (`KismetMathLibrary.BreakDateTime` (`KismetMathLibrary.Now`)))
  (`ModAPI.LogMessage` (`ModAPI.GetModAPI`) (`KismetStringLibrary.Concat_StrStr` "[" (`KismetStringLibrary.Conv_IntToString` _year) "-" (`KismetStringLibrary.Conv_IntToString` _month) "-" (`KismetStringLibrary.Conv_IntToString` _day) " " (`KismetStringLibrary.Conv_IntToString` _hour) ":" (`KismetStringLibrary.Conv_IntToString` _minute) ":" (`KismetStringLibrary.Conv_IntToString` _second) "." (`KismetStringLibrary.Conv_IntToString` _millisecond) "] [" `Mod Name` "]" Message)))

(fn `Set Dilation From Option`
  (params (Option :type String))
  (returns (Dilation :type "Float (double-precision)"))
  (bind _output_get (set `self.SetTimeDilation` (`KismetStringLibrary.Conv_StringToDouble` (`KismetStringLibrary.LeftChop` Option 1))))
  (return _output_get))

(fn `UserConstructionScript`)