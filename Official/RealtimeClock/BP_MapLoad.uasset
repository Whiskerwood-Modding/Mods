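; BP_MapLoad injects a clock indicator widget into an existing UI when the map begins play.
; After a short delay it scans all user widgets for one named TimeControlButtons.
; It walks two parents up to that widget's VerticalBox, then creates a WBP_ClockIndicator for the first player and adds it as a child, hooking into UI by object name rather than editing it.
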(event `self.ReceiveBeginPlay`
  (`KismetSystemLibrary.Delay` 0.2)
  (bind _foundwidgets (`WidgetBlueprintLibrary.GetAllWidgetsOfClass` "/Script/UMG.UserWidget" false))
  (for _array_element _foundwidgets
    (if (== (`KismetSystemLibrary.GetObjectName` _array_element) "TimeControlButtons")
      (bind _asvertical_box (cast `VerticalBox` (`Widget.GetParent` (`Widget.GetParent` _array_element))))
      (bind _returnvalue (`|CreateWidget` "/Game/Mods/RealtimeClock/WBP_ClockIndicator.WBP_ClockIndicator_C" (`GameplayStatics.GetPlayerController` 0)))
      (`PanelWidget.AddChild` _asvertical_box _returnvalue))))

(fn `UserConstructionScript`)