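; BP_MapLoad is the map-load Blueprint for the CheatMode mod, giving access to a developer cheat menu.
; Once the mod API signals that loading has finished, it enables player input and creates the Arcoview_developer_BP widget.
; The L key alternately adds that widget to the viewport and removes it through a FlipFlop.
; An author comment warns that the mod can brick saves and is meant only for temporary ones.
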(event `self.ReceiveBeginPlay`
  ; WARNING: THIS MOD CAN BRICK YOUR SAVE! ONLY USE ON TEMP SAVES!
  (add `ModAPI.onLoadingFinished` (`ModAPI.GetModAPI`) (delegate `OnLoadingFinished`)))

(event `OnLoadingFinished`
  ; WARNING: THIS MOD CAN BRICK YOUR SAVE! ONLY USE ON TEMP SAVES!
  (`self.EnableInput` (`GameplayStatics.GetPlayerController` 0))
  (bind _returnvalue (`|CreateWidget` "/Game/UI/ArcoViews/Arcoview_developer_BP.Arcoview_developer_BP_C"))
  (set `self.CheatMenuRef` _returnvalue))

(event `Key|L`
  (params (Key :type "Key Structure"))
  (bind _cheatmenuref (`self.CheatMenuRef`))
  ; WARNING: THIS MOD CAN BRICK YOUR SAVE! ONLY USE ON TEMP SAVES!
  (:`Pressed`
    (`/Engine/EditorBlueprintResources/StandardMacros.FlipFlop`
      (:`A`
        (`UserWidget.AddToViewport` _cheatmenuref -1))
      (:`B`
        (`Widget.RemoveFromParent` _cheatmenuref)))))

(fn `UserConstructionScript`)